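; BP_Goal is the level exit that ends the game with a win when an eligible player reaches it.
; On overlap with its Cube, it checks that an AT_Character's player state holds both keys or has killed all guards.
; If so, it sets the game state enum, pauses the game and shows the win widget.
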(event `self.Cube.OnComponentBeginOverlap`
  (params (OverlappedComponent :type "PrimitiveComponent Object Reference") (OtherActor :type "Actor Object Reference") (OtherComp :type "PrimitiveComponent Object Reference") (OtherBodyIndex :type Integer) (bFromSweep :type Boolean) (SweepResult :type "HitResult Structure (by ref)"))
  (bind _asat_character (cast `/Game/Character/AT_Char/AT_Character` OtherActor))
  (bind _asbp_atplayer_state (cast `/Game/System/BP_ATPlayerState` (`Pawn.PlayerState` _asat_character)))
  (if (or (and (`/Game/System/BP_ATPlayerState.Key1` _asbp_atplayer_state) (`/Game/System/BP_ATPlayerState.Key2` _asbp_atplayer_state)) (`/Game/System/BP_ATPlayerState.KilledAllGuards` _asbp_atplayer_state))
    (bind _asbp_atgame_state (cast `/Game/System/BP_ATGameState` (`GameplayStatics.GetGameState`)))
    (set `/Game/System/BP_ATGameState.GameState` "NewEnumerator4" _asbp_atgame_state)
    (`GameplayStatics.SetGamePaused` true)
    (bind _returnvalue (`|CreateWidget` "/Game/System/Widget/BP_WinWidget.BP_WinWidget_C"))
    (`UserWidget.AddToViewport` _returnvalue 0)))

(fn `UserConstructionScript`)