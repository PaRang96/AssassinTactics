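; Game state Blueprint that tracks a guard count and can open the in-game HUD widget.
; Tick prints the current GameState enum every frame as a debug readout, and OpenInGameWidget creates BP_InGameWidget and adds it to the viewport.
; DeductGuardsNum decrements the count, but its zero check leads nowhere and KilledAllGuards is empty.
; The guard-counting setup and the code setting the player state's KilledAllGuards flag are disconnected and never run.
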(event `self.ReceiveBeginPlay`)

(event `self.ReceiveTick`
  (params (DeltaSeconds :type "Float (single-precision)"))
  (`KismetSystemLibrary.PrintString` (`|GetEnumeratorNameAsString` (`self.GameState`)) true true (struct :`G` 0.66 :`B` 1.0 :`A` 1.0) DeltaSeconds))

(fn `DeductGuardsNum`
  (bind _result (`/Engine/EditorBlueprintResources/StandardMacros.DecrementInt` (`self.GuardsNum`))
    (:`  `
      (if (== _result 0)
        _))))

(fn `KilledAllGuards`)

(fn `OpenInGameWidget`
  (bind _returnvalue (`|CreateWidget` "/Game/System/Widget/BP_InGameWidget.BP_InGameWidget_C"))
  (`UserWidget.AddToViewport` _returnvalue 0))

(fn `UserConstructionScript`)