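; BP_Inventory tracks the player's counts of three items: liquor, rocks and smoke shells.
; Obtain events increment a count, Use functions decrement it, and both push the number to that item's in-game widget.
; Using an item also notifies BP_ATPlayerState of the first player controller through a per-item consume message.
; Check functions report whether at least one is held, but Use functions do not call them; Consume functions are empty stubs.
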(event `self.ReceiveBeginPlay`
  (`/Engine/EditorBlueprintResources/StandardMacros.IsValid` (`self.InGameWidget`)))

(event `/Game/System/BPI_ItemInterface.ObtainLiquor`
  (`KismetSystemLibrary.PrintString` "obtain liquor")
  (`self.GetLiquor`))

(event `/Game/System/BPI_ItemInterface.ObtainRock`
  (`KismetSystemLibrary.PrintString` "obtain rock")
  (`self.GetRock`))

(event `/Game/System/BPI_ItemInterface.ObtainSmokeShell`
  (`KismetSystemLibrary.PrintString` "obtain shell")
  (`self.GetSmokeShell`))

(fn `CheckLiquorNum`
  (returns (CanUseLiquor :type Boolean))
  (return (>= (`self.LiquorNum`) 1)))

(fn `CheckSmokeShellNum`
  (returns (CanUseSmokeShell :type Boolean))
  (return (>= (`self.SmokeShellNum`) 1)))

(fn `ChekRockNum`
  (returns (CanUseRock :type Boolean))
  (return (>= (`self.RockNum`) 1)))

(fn `ConsumeLiquor`)

(fn `ConsumeRock`)

(fn `ConsumeSmokeShell`)

(fn `GetLiquor`
  (bind _result (`/Engine/EditorBlueprintResources/StandardMacros.IncrementInt` (`self.LiquorNum`))
    (:`  `
      (`self.UpdateLiquor` _result))))

(fn `GetRock`
  (bind _result (`/Engine/EditorBlueprintResources/StandardMacros.IncrementInt` (`self.RockNum`))
    (:`  `
      (`self.UpdateRock` _result))))

(fn `GetSmokeShell`
  (bind _result (`/Engine/EditorBlueprintResources/StandardMacros.IncrementInt` (`self.SmokeShellNum`))
    (:`  `
      (`self.UpdateSmokeShell` _result))))

(fn `UpdateLiquor`
  (params (LiquorNumber :type Integer))
  (`/Game/System/Widget/SubWidgets/InGameSubwidget/BP_LiquorWidget.SetLiquorInfo` (`/Game/System/Widget/BP_InGameWidget.BP_LiquorWidget` (`self.InGameWidget`)) LiquorNumber))

(fn `UpdateRock`
  (params (RockNumber :type Integer))
  (`/Game/System/Widget/SubWidgets/InGameSubwidget/BP_RockWidget.SetRockInfo` (`/Game/System/Widget/BP_InGameWidget.BP_RockWidget` (`self.InGameWidget`)) RockNumber))

(fn `UpdateSmokeShell`
  (params (SmokeShellNum :type Integer))
  (`/Game/System/Widget/SubWidgets/InGameSubwidget/BP_SmokeShellWidget.SetSmokeShellInfo` (`/Game/System/Widget/BP_InGameWidget.BP_SmokeShellWidget` (`self.InGameWidget`)) SmokeShellNum))

(fn `UseLiquor`
  (bind _result (`/Engine/EditorBlueprintResources/StandardMacros.DecrementInt` (`self.LiquorNum`))
    (:`  `
      (`self.UpdateLiquor` _result)
      (bind _asbp_atplayer_state (cast `/Game/System/BP_ATPlayerState` (`Controller.PlayerState` (`GameplayStatics.GetPlayerController` 0))))
      (message `/Game/System/BPI_ItemInterface.ConsumeLiquor` _asbp_atplayer_state))))

(fn `UserConstructionScript`)

(fn `UseRock`
  (bind _result (`/Engine/EditorBlueprintResources/StandardMacros.DecrementInt` (`self.RockNum`))
    (:`  `
      (`self.UpdateRock` _result)
      (bind _asbp_atplayer_state (cast `/Game/System/BP_ATPlayerState` (`Controller.PlayerState` (`GameplayStatics.GetPlayerController` 0))))
      (message `/Game/System/BPI_ItemInterface.ConsumeRock` _asbp_atplayer_state))))

(fn `UseSmokeShell`
  (bind _result (`/Engine/EditorBlueprintResources/StandardMacros.DecrementInt` (`self.SmokeShellNum`))
    (:`  `
      (`self.UpdateSmokeShell` _result)
      (bind _asbp_atplayer_state (cast `/Game/System/BP_ATPlayerState` (`Controller.PlayerState` (`GameplayStatics.GetPlayerController` 0))))
      (message `/Game/System/BPI_ItemInterface.ConsumeSmokeShell` _asbp_atplayer_state))))