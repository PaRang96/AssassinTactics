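; BP_SoundRock is a thrown rock actor that makes a noise, reported to AI hearing.
; On BeginPlay it throws itself, activating projectile movement with its Velocity variable scaled by distance.
; After a fixed short delay, rather than on impact, it plays a bonk sound and reports a noise event at the mesh location with ATCharacter as instigator.
; It then sets a short lifespan to remove itself.
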(event `Throw`
  (params (Velocity :type "Vector Structure"))
  (bind _projectilemovement (`self.ProjectileMovement`))
  (bind _returnvalue (`SceneComponent.K2_GetComponentLocation` (`self.StaticMesh`)))
  (set `MovementComponent.Velocity` (* Velocity (* (`self.DIstance`) 1.8)) _projectilemovement)
  (`ActorComponent.Activate` _projectilemovement false)
  (`KismetSystemLibrary.Delay` 0.5)
  (`GameplayStatics.PlaySoundAtLocation` "/Game/AI/Sound/bonk-sound-effect-36055__online-audio-converter_com_.bonk-sound-effect-36055__online-audio-converter_com_" _returnvalue (struct) 1.0 1.0 0.0 null null null)
  (`AISense_Hearing.ReportNoiseEvent` _returnvalue 1.0 (`self.AT_Character`))
  (`self.SetLifeSpan` 3.0))

(event `self.ReceiveBeginPlay`
  (`self.Throw` (`self.Velocity`)))

(fn `UserConstructionScript`)