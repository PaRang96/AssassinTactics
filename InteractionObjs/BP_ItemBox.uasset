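; BP_ItemBox is a pickup box that grants a random item (Liquor, Smoke Shell or Rock) when anything overlaps its Box.
; The overlap rolls the item enum, finds BP_Inventory with GetActorOfClass and calls the matching Obtain message on it.
; Deactivate then hides the Cube and disables collision on Cube and Box instead of destroying the actor.
; Its own Obtain and ConsumeLiquor functions are empty stubs.
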(event `self.Box.OnComponentBeginOverlap`
  (params (OverlappedComponent :type "PrimitiveComponent Object Reference") (OtherActor :type "Actor Object Reference") (OtherComp :type "PrimitiveComponent Object Reference") (OtherBodyIndex :type Integer) (bFromSweep :type Boolean) (SweepResult :type "HitResult Structure (by ref)"))
  (bind _returnvalue (`GameplayStatics.GetActorOfClass` "/Game/System/BP_Inventory.BP_Inventory_C"))
  (bind _output_get (set `self.Item` (cast `/Game/IteractionObjs/EN_Item` (`KismetMathLibrary.Conv_IntToByte` (`KismetMathLibrary.RandomIntegerInRange` 0 2)))))
  (switch `/Game/IteractionObjs/EN_Item` _output_get
    (:`NewEnumerator0`
      (message `/Game/System/BPI_ItemInterface.ObtainLiquor` _returnvalue)
      (`self.Deactivate`))
    (:`NewEnumerator1`
      (message `/Game/System/BPI_ItemInterface.ObtainSmokeShell` _returnvalue)
      (`self.Deactivate`))
    (:`NewEnumerator2`
      (message `/Game/System/BPI_ItemInterface.ObtainRock` _returnvalue)
      (`self.Deactivate`))))

(fn `ConsumeLiquor`
  (return))

(fn `Deactivate`
  (`SceneComponent.SetVisibility` (`self.Cube`) false false)
  (`PrimitiveComponent.SetCollisionEnabled` (`self.Cube`) "NoCollision")
  (`PrimitiveComponent.SetCollisionEnabled` (`self.Box`) "NoCollision"))

(fn `ObtainLiquor`)

(fn `ObtainRock`)

(fn `ObtainSmokeShell`)

(fn `UserConstructionScript`)